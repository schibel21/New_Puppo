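; PeleBP is a flipbook-animated person NPC that patrols along the X axis, approaches the BPpuppo dog and pets it.
; Each Tick, MoveLogic paces it back and forth, flipping direction on capsule hits, or chases the dog inside DetectionRadius unless it is invincible, barking, sniffing, hiding or begging.
; PetLogic separately switches from the walk to the petting flipbook when the first BPpuppo found is close and not hiding.
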(event OnComponentHit(CapsuleComponent)
  (params (HitComponent :type Primitive%20Component%20Object%20Reference) (OtherActor :type Actor%20Object%20Reference) (OtherComp :type Primitive%20Component%20Object%20Reference) (NormalImpulse :type Vector :default "0, 0, 0") (Hit :type Hit%20Result%20Structure%20%28by%20ref%29))
  (if (Variables|Default|GetmovingRight)
    (Variables|Default|SetmovingRight false)
    (else
      (Variables|Default|SetmovingRight true))))

(event OnComponentBeginOverlap(detectionRadius)
  (params (OverlappedComponent :type Primitive%20Component%20Object%20Reference) (OtherActor :type Actor%20Object%20Reference) (OtherComp :type Primitive%20Component%20Object%20Reference) (OtherBodyIndex :type Integer) (bFromSweep :type Boolean) (SweepResult :type Hit%20Result%20Structure%20%28by%20ref%29))
  (Utilities|Casting|CastToBPpuppo OtherActor)
  (Variables|Default|SetinRange true))

(event OnComponentEndOverlap(detectionRadius)
  (params (OverlappedComponent :type Primitive%20Component%20Object%20Reference) (OtherActor :type Actor%20Object%20Reference) (OtherComp :type Primitive%20Component%20Object%20Reference) (OtherBodyIndex :type Integer))
  (Utilities|Casting|CastToBPpuppo OtherActor)
  (Variables|Default|SetinRange false))

(event EventTick
  (params (DeltaSeconds :type Float%20%28single-precision%29))
  (CallFunction|MoveLogic)
  (CallFunction|PetLogic))

(fn ConstructionScript)

(fn MovePerson
  (params (speedModifier :type Float%20%28single-precision%29))
  (Pawn|Input|AddMovementInput (Math|Vector|MakeVector (* 1 speedModifier) 0.0 0.0) 1.0 false))

(fn MoveLogic
  (bind _capsulecomponent (Variables|Collision|GetCapsuleComponent))
  (bind _capsulecomponent_2 (Variables|Collision|GetCapsuleComponent))
  (bind _capsulecomponent_3 (Variables|Collision|GetCapsuleComponent))
  (if (Variables|Default|GetinRange)
    (bind _outactors (Actor|GetAllActorsOfClass "/Game/Puppo/BPpuppo.BPpuppo_C"))
    (if (Math|Boolean|ORBoolean (Variables|/Game/Puppo/BPpuppo.BPpuppo_C|Getinvincible (Utilities|Array|Get(acopy) _outactors)) (Variables|/Game/Puppo/BPpuppo.BPpuppo_C|Getbarking (Utilities|Array|Get(acopy) _outactors)) (Variables|/Game/Puppo/BPpuppo.BPpuppo_C|Getsniffing (Utilities|Array|Get(acopy) _outactors)) (Variables|/Game/Puppo/BPpuppo.BPpuppo_C|Gethiding (Utilities|Array|Get(acopy) _outactors)) (Variables|/Game/Puppo/BPpuppo.BPpuppo_C|Getbegging (Utilities|Array|Get(acopy) _outactors)))
      (if (Variables|Default|GetmovingRight) :!label _label
        (Transformation|SetWorldRotation _capsulecomponent_3 "0,180.000000, 0" false false)
        (CallFunction|MovePerson 0.5)
        (else
          (Transformation|SetWorldRotation _capsulecomponent_3 "0,0.000000, 0" false false)
          (CallFunction|MovePerson -0.5)))
      (elif (> (Math|Float|Absolute(Float) (- (.X (Math|Vector|BreakVector (Transformation|GetActorLocation))) (.X (Math|Vector|BreakVector (Transformation|GetActorLocation (Utilities|Array|Get(acopy) _outactors)))))) 9e+01)
        (if (> (.X (Math|Vector|BreakVector (Transformation|GetActorLocation (Utilities|Array|Get(acopy) _outactors)))) (.X (Math|Vector|BreakVector (Transformation|GetWorldLocation (Variables|Collision|GetCapsuleComponent)))))
          (CallFunction|MovePerson 0.8)
          (Variables|Default|SetmovingRight true)
          (Transformation|SetWorldRotation _capsulecomponent "0,180.000000, 0" false false)
          (else
            (CallFunction|MovePerson -0.8)
            (Variables|Default|SetmovingRight false)
            (Transformation|SetWorldRotation _capsulecomponent "0,0.000000, 0" false false)))
        (elif (> (.X (Math|Vector|BreakVector (Transformation|GetActorLocation (Utilities|Array|Get(acopy) _outactors)))) (.X (Math|Vector|BreakVector (Transformation|GetWorldLocation (Variables|Collision|GetCapsuleComponent)))))
          (Transformation|SetWorldRotation _capsulecomponent_2 "0,180.000000, 0" false false)
          (else
            (Transformation|SetWorldRotation _capsulecomponent_2 "0,0.000000, 0" false false)))))
    (else
      (goto _label))))

(fn PetLogic
  (bind _sprite (Variables|Default|GetSprite))
  (bind _outactors (Actor|GetAllActorsOfClass "/Game/Puppo/BPpuppo.BPpuppo_C"))
  (if (<= (Math|Float|Absolute(Float) (- (.X (Math|Vector|BreakVector (Transformation|GetActorLocation (Utilities|Array|Get(acopy) _outactors)))) (.X (Math|Vector|BreakVector (Transformation|GetActorLocation))))) 9e+01)
    (if (Variables|/Game/Puppo/BPpuppo.BPpuppo_C|Gethiding (Utilities|Array|Get(acopy) _outactors))
      (Sprite|SetFlipbook _sprite "/Game/Person/Animations/HUMAN_WALK/PELE_WALK.PELE_WALK" :!label _label)
      (else
        (Sprite|SetFlipbook _sprite "/Game/Person/Animations/HUMAN_PETS/PET_PELE.PET_PELE")))
    (else
      (goto _label))))